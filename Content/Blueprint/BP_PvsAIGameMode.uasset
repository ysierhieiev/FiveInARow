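; Game mode for a player-versus-AI match of a line-forming board game.
; On BeginPlay it reads the difficulty from the game instance, spawns a grid of BP_Chunk tiles and caches the player controller.
; AIMove places the AI's shape, plays a sound, then either ends the round on a winning line or records the move, checks for a draw and re-enables player input.
; The draw check assumes a 64-cell board.
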(event `self.ReceiveBeginPlay`
  ;[1 1 1] Start
  (bind _asbp_game_instance (cast `/Game/Blueprint/BP_GameInstance` (`GameplayStatics.GetGameInstance`)))
  (set `self.Difficult` (`/Game/Blueprint/BP_GameInstance.DifficultOfGame` _asbp_game_instance))
  (`self.CreateGameTable`)
  (bind _asbp_player_controller (cast `/Game/Blueprint/BP_PlayerController` (`GameplayStatics.GetPlayerController` 0)))
  (set `self.PlayerController` _asbp_player_controller))

(fn `AIMove`
  (bind _returnvalue (`self.PCMove`))
  (bind _statusdemonstration (`Chunk.StatusDemonstration` _returnvalue))
  (`StaticMeshComponent.SetStaticMesh` _statusdemonstration "/Game/Meshes/AI_Shape.AI_Shape")
  (`GameplayStatics.PlaySoundAtLocation` "/Game/Sounds/SoundMove.SoundMove" (`SceneComponent.K2_GetComponentLocation` _statusdemonstration) (struct) 1.0 1.0 0.0 null null null)
  (bind _yposition (`Chunk.Yposition` _returnvalue))
  (bind _xposition (`Chunk.Xposition` _returnvalue))
  (bind _returnvalue_2 (`self.isWin` _yposition _xposition (`self.WinLineCount`)))
  (if _returnvalue_2
    (set `self.ResultOfRound` "RR_WinAI")
    (bind _returnvalue_3 (`|CreateWidget` "/Game/Blueprint/UMG/WBEndRound.WBEndRound_C"))
    (`UserWidget.AddToViewport` _returnvalue_3 0)
    (else
      (`self.AddToMoveMemory` _yposition _xposition)
      (`self.isTableIsFull`)
      (set `/Game/Blueprint/BP_PlayerController.CanStep` true (`self.PlayerController`)))))

(fn `CreateGameTable`
  (`KismetArrayLibrary.Array_Clear` (`self.ChunkOfRows`))
  (for _index (range (`self.MaxBoardSize`))
    (`KismetArrayLibrary.Array_Add` (`self.ChunkOfRows`))
    (for _index_2 (range (`self.MaxBoardSize`))
      (bind _output_get (set `self.Location` (`KismetMathLibrary.MakeTransform` (`KismetMathLibrary.MakeVector` (`self.X`) (`self.Y`) 10.0))))
      (bind _returnvalue (`|SpawnActorFromClass` "/Game/Blueprint/BP_Chunk.BP_Chunk_C" _output_get "Undefined" "OverrideRootScale" null null))
      (`self.AddToCol` _index _returnvalue)
      (`Chunk.SetPositionInBoard` _returnvalue _index_2 _index)
      (set `self.Y` (+ (`self.Y`) 110.0)))
    (set `self.X` (- (`self.X`) 110.0))
    (set `self.Y` -400.0)))

(fn `isTableIsFull`
  (if (== (`self.FillChunksCount`) 64)
    (set `self.ResultOfRound` "RR_Draw")
    (bind _returnvalue (`|CreateWidget` "/Game/Blueprint/UMG/WBEndRound.WBEndRound_C"))
    (`UserWidget.AddToViewport` _returnvalue 0)))

(fn `UserConstructionScript`)