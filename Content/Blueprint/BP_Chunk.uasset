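; BP_Chunk is one clickable board cell in a turn-based line-forming game against an AI.
; Cursor hover previews the player's shape on empty cells while the player can step, using a status enum.
; Clicking claims the cell, locks input and plays a sound and placement timeline.
; When that finishes, the game mode checks for a win, showing the end-round widget, or checks board fullness, records the move and triggers the AI.
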(event `self.ReceiveBeginPlay`
  (bind _asbp_player_controller (cast `/Game/Blueprint/BP_PlayerController` (`GameplayStatics.GetPlayerController` 0)))
  (set `self.Player` _asbp_player_controller)
  (bind _asbp_pvs_aigame_mode (cast `/Game/Blueprint/BP_PvsAIGameMode` (`GameplayStatics.GetGameMode`)))
  (set `self.GameMode` _asbp_pvs_aigame_mode))

(event `self.MeshComp.OnBeginCursorOver`
  (params (TouchedComponent :type "PrimitiveComponent Object Reference"))
  (if (and (`/Game/Blueprint/BP_PlayerController.CanStep` (`self.Player`)) (`|EnumEquality` (`self.CurrentChunkStatus`) "CS_Empty"))
    (`StaticMeshComponent.SetStaticMesh` (`self.StatusDemonstration`) "/Game/Meshes/Player_Shape_Projection.Player_Shape_Projection")
    (set `self.CurrentChunkStatus` "CS_Player_Projection")))

(event `self.MeshComp.OnEndCursorOver`
  (params (TouchedComponent :type "PrimitiveComponent Object Reference"))
  (if (and (`/Game/Blueprint/BP_PlayerController.CanStep` (`self.Player`)) (`|EnumEquality` (`self.CurrentChunkStatus`) "CS_Player_Projection"))
    (`StaticMeshComponent.SetStaticMesh` (`self.StatusDemonstration`) null)
    (set `self.CurrentChunkStatus` "CS_Empty")))

(event `self.MeshComp.OnClicked`
  (params (TouchedComponent :type "PrimitiveComponent Object Reference") (ButtonPressed :type "Key Structure"))
  (bind _gamemode (`self.GameMode`))
  (bind _gamemode_2 (`self.GameMode`))
  (bind _xposition (`self.Xposition`))
  (bind _yposition (`self.Yposition`))
  (bind _player (`self.Player`))
  (if (and (`/Game/Blueprint/BP_PlayerController.CanStep` _player) (`|EnumEquality` (`self.CurrentChunkStatus`) "CS_Player_Projection"))
    (`StaticMeshComponent.SetStaticMesh` (`self.StatusDemonstration`) "/Game/Meshes/Player_Shape.Player_Shape")
    (set `/Game/Blueprint/BP_PlayerController.CanStep` false _player)
    (set `self.CurrentChunkStatus` "CS_Player")
    (`GameplayStatics.PlaySoundAtLocation` "/Game/Sounds/SoundMove.SoundMove" (0.0 0.0 105.0) (struct) 1.0 1.0 0.0 null null null)
    (bind (_direction _rotationpitch _location) (`Timeline|SetAnimation`)
      (:`Update`
        (`SceneComponent.K2_SetRelativeLocationAndRotation` (`self.StatusDemonstration`) _location (`KismetMathLibrary.MakeRotator` 0.0 _rotationpitch) false false))
      (:`Finished`
        (`/Engine/EditorBlueprintResources/StandardMacros.IncrementInt` (`PvsAIGameMode.FillChunksCount` _gamemode_2)
          (:`  `
            (bind _returnvalue (`PvsAIGameMode.isWin` _gamemode_2 _yposition _xposition (`PvsAIGameMode.WinLineCount` _gamemode_2)))
            (if _returnvalue
              (set `PvsAIGameMode.ResultOfRound` "RR_WinPlayer" _gamemode)
              (bind _returnvalue_2 (`|CreateWidget` "/Game/Blueprint/UMG/WBEndRound.WBEndRound_C"))
              (`UserWidget.AddToViewport` _returnvalue_2 0)
              (else
                (`/Game/Blueprint/BP_PvsAIGameMode.isTableIsFull` _gamemode)
                (`PvsAIGameMode.AddToMoveMemory` _gamemode _yposition _xposition true)
                (`/Game/Blueprint/BP_PvsAIGameMode.AIMove` _gamemode)))))))))

(event `self.SetEmptyMesh`
  (`StaticMeshComponent.SetStaticMesh` (`self.StatusDemonstration`) null))

(fn `UserConstructionScript`)